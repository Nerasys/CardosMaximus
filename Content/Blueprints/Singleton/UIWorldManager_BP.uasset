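; UIWorldManager_BP is a singleton manager that owns the root UI widget and exposes events for pushing menus and prompts onto it.
; On init it waits briefly, registers itself on the GameManager game instance, then creates UI_Base without a world context and opens the login/register menu.
; Its push events forward collection menu, login, register and generic prompt requests to that UI_Base.
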(event Custom|PushPrompt
  (params (InPromptText :type Text) (InPromptOwner :type UI%20Login%20Register%20Object%20Reference) (InPromptIndex :type Integer))
  (Default|PushPrompt (Variables|Default|GetUI_Base) InPromptText InPromptOwner InPromptIndex))

(event Custom|Push%20CollectionMenu
  (Default|PushMenuCollection (Variables|Default|GetUI_Base)))

(event Custom|Push%20Login%20Prompt
  (Default|PushPromptLogin (Variables|Default|GetUI_Base)))

(event Custom|Push%20Register%20Prompt
  (Default|PushPromptRegister (Variables|Default|GetUI_Base)))

(event EventInitBP
  (Utilities|FlowControl|Delay 0.2)
  (bind _returnvalue (Class|UIWorldManager|GetNoContextGameInstance))
  (bind _asgame_manager (Utilities|Casting|CastToGameManager _returnvalue))
  (Variables|Default|SetGameMgr _asgame_manager)
  (Variables|/Game/Blueprints/Singleton/GameManager.GameManager_C|SetWorldUIMgr _asgame_manager self)
  (bind _returnvalue_2 (Default|CreateWidgetWithoutContext (Variables|Default|GetGameMgr) "/Game/UI/UI_Base.UI_Base_C"))
  (bind _asui_base (Utilities|Casting|CastToUI_Base _returnvalue_2))
  (bind _output_get (Variables|Default|SetUI_Base _asui_base))
  (UserInterface|Viewport|AddtoViewport _output_get 0)
  (Default|PushMenu (Variables|Default|GetUI_Base) "/Game/UI/MainUI/UI_LoginRegister.UI_LoginRegister_C"))